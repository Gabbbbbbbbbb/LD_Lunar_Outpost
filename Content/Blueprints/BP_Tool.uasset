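; BP_Tool is a pickup item that the player collects to mark the tool as owned on BP_Engine.
; Sphere overlap events track whether the player is in range and show or hide an interact button widget on the third-person character.
; Tick polls the character's Interact flag and, when set in range, hides the prompt, sets the engine's ToolOwned through GetActorOfClass, and destroys the actor.
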(event `self.ReceiveTick`
  (params (DeltaSeconds :type "Float (single-precision)"))
  (if (not (`self.IsPickedUp`))
    (bind _returnvalue (`GameplayStatics.GetActorOfClass` "/Game/ThirdPerson/Blueprints/BP_ThirdPersonCharacter.BP_ThirdPersonCharacter_C"))
    (if (`/Game/ThirdPerson/Blueprints/BP_ThirdPersonCharacter.Interact` _returnvalue)
      (if (`self.inArea`)
        (set `self.IsPickedUp` true)
        (`/Game/ThirdPerson/Blueprints/BP_ThirdPersonCharacter.Widget_Interact_Disappear` (cast `/Game/ThirdPerson/Blueprints/BP_ThirdPersonCharacter` (`GameplayStatics.GetPlayerCharacter` 0) :!pure true) null)
        (bind _returnvalue_2 (`GameplayStatics.GetActorOfClass` "/Game/Blueprints/BP_Engine.BP_Engine_C"))
        (set `/Game/Blueprints/BP_Engine.ToolOwned` true _returnvalue_2)
        (`self.K2_DestroyActor`)))))

(event `self.Sphere.OnComponentBeginOverlap`
  (params (OverlappedComponent :type "PrimitiveComponent Object Reference") (OtherActor :type "Actor Object Reference") (OtherComp :type "PrimitiveComponent Object Reference") (OtherBodyIndex :type Integer) (bFromSweep :type Boolean) (SweepResult :type "HitResult Structure (by ref)"))
  (if (== OtherActor (`GameplayStatics.GetPlayerCharacter` 0))
    (if (not (`self.IsPickedUp`))
      (set `self.inArea` true)
      (`/Game/ThirdPerson/Blueprints/BP_ThirdPersonCharacter.Widget_Interact_Appear` (cast `/Game/ThirdPerson/Blueprints/BP_ThirdPersonCharacter` (`GameplayStatics.GetPlayerCharacter` 0) :!pure true) "/Game/Widget/WBP_InteractButton.WBP_InteractButton_C"))))

(event `self.Sphere.OnComponentEndOverlap`
  (params (OverlappedComponent :type "PrimitiveComponent Object Reference") (OtherActor :type "Actor Object Reference") (OtherComp :type "PrimitiveComponent Object Reference") (OtherBodyIndex :type Integer))
  (if (== OtherActor (`GameplayStatics.GetPlayerCharacter` 0))
    (set `self.inArea` false)
    (`/Game/ThirdPerson/Blueprints/BP_ThirdPersonCharacter.Widget_Interact_Disappear` (cast `/Game/ThirdPerson/Blueprints/BP_ThirdPersonCharacter` (`GameplayStatics.GetPlayerCharacter` 0) :!pure true) null)))

(fn `UserConstructionScript`)