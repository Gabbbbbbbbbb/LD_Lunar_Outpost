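; Camera switch actor that changes player 0's view target when BP_ThirdPersonCharacter overlaps one of two triggers, InBox or OutBox.
; InBox switches the view to CamIn, while OutBox switches to either the character's own view or CamOut, depending on the CameraPlayer flag.
; Each switch also calls the character's Delay and sets its InCamArea flag, which is false only for the CamOut switch.
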(event `self.InBox.OnActorBeginOverlap`
  (params (OverlappedActor :type "Actor Object Reference") (OtherActor :type "Actor Object Reference"))
  ;[0.1146 0.1146 0.1146] New camera forward (In)
  (bind _asbp_third_person_character (cast `/Game/ThirdPerson/Blueprints/BP_ThirdPersonCharacter` OtherActor))
  (`PlayerController.SetViewTargetWithBlend` (`GameplayStatics.GetPlayerController` 0) (`self.CamIn`) 0.0 "VTBlend_Linear" 0.0 false)
  (set `/Game/ThirdPerson/Blueprints/BP_ThirdPersonCharacter.InCam_Area` true _asbp_third_person_character)
  (`/Game/ThirdPerson/Blueprints/BP_ThirdPersonCharacter.Delay` _asbp_third_person_character))

(event `self.OutBox.OnActorBeginOverlap`
  (params (OverlappedActor :type "Actor Object Reference") (OtherActor :type "Actor Object Reference"))
  (bind _returnvalue (`GameplayStatics.GetPlayerController` 0))
  (bind _asbp_third_person_character (cast `/Game/ThirdPerson/Blueprints/BP_ThirdPersonCharacter` OtherActor))
  (if (`self.CameraPlayer`)
    (`PlayerController.SetViewTargetWithBlend` _returnvalue _asbp_third_person_character 0.0 "VTBlend_Linear" 0.0 false)
    (`/Game/ThirdPerson/Blueprints/BP_ThirdPersonCharacter.Delay` _asbp_third_person_character)
    (set `/Game/ThirdPerson/Blueprints/BP_ThirdPersonCharacter.InCam_Area` true _asbp_third_person_character)
    (else
      (`PlayerController.SetViewTargetWithBlend` _returnvalue (`self.CamOut`) 0.0 "VTBlend_Linear" 0.0 false)
      (`/Game/ThirdPerson/Blueprints/BP_ThirdPersonCharacter.Delay` _asbp_third_person_character)
      (set `/Game/ThirdPerson/Blueprints/BP_ThirdPersonCharacter.InCam_Area` false _asbp_third_person_character))))

(fn `UserConstructionScript`)