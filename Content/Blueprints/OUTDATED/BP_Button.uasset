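; BP_Button is an interactable button that toggles a referenced door open and closed.
; Its sphere overlap flags the button as usable and shows or hides an interact prompt widget through the player character.
; Tick polls the character's Interact flag and, while usable, flips the door on every tick that flag is true.
; Opening hides the door's cube and disables its collision, and closing restores both.
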(event `self.Sphere.OnComponentBeginOverlap`
  (params (OverlappedComponent :type "PrimitiveComponent Object Reference") (OtherActor :type "Actor Object Reference") (OtherComp :type "PrimitiveComponent Object Reference") (OtherBodyIndex :type Integer) (bFromSweep :type Boolean) (SweepResult :type "HitResult Structure (by ref)"))
  (set `self.IsOK` true)
  (`/Game/ThirdPerson/Blueprints/BP_ThirdPersonCharacter.Widget_Interact_Appear` (cast `/Game/ThirdPerson/Blueprints/BP_ThirdPersonCharacter` (`GameplayStatics.GetPlayerCharacter` 0) :!pure true) "/Game/Widget/WBP_InteractButton.WBP_InteractButton_C"))

(event `self.Sphere.OnComponentEndOverlap`
  (params (OverlappedComponent :type "PrimitiveComponent Object Reference") (OtherActor :type "Actor Object Reference") (OtherComp :type "PrimitiveComponent Object Reference") (OtherBodyIndex :type Integer))
  (set `self.IsOK` false)
  (`/Game/ThirdPerson/Blueprints/BP_ThirdPersonCharacter.Widget_Interact_Disappear` (cast `/Game/ThirdPerson/Blueprints/BP_ThirdPersonCharacter` (`GameplayStatics.GetPlayerCharacter` 0) :!pure true) null))

(event `self.ReceiveTick`
  (params (DeltaSeconds :type "Float (single-precision)"))
  (bind _returnvalue (`GameplayStatics.GetActorOfClass` "/Game/ThirdPerson/Blueprints/BP_ThirdPersonCharacter.BP_ThirdPersonCharacter_C"))
  (if (`/Game/ThirdPerson/Blueprints/BP_ThirdPersonCharacter.Interact` _returnvalue)
    (if (`self.IsOK`)
      (if (`self.IsOpen`)
        (`self.Close` (`self.Door`))
        (set `self.IsOpen` false)
        (else
          (`self.Open` (`self.Door`))
          (set `self.IsOpen` true))))))

(fn `Close`
  (params (Door :type "/Game/Blueprints/BP_DoorOudated Object Reference"))
  (bind _cube (`/Game/Blueprints/BP_DoorOudated.Cube` Door))
  (`SceneComponent.SetVisibility` _cube true false)
  (`PrimitiveComponent.SetCollisionEnabled` _cube "QueryAndPhysics")
  (return))

(fn `Open`
  (params (Door :type "/Game/Blueprints/BP_DoorOudated Object Reference"))
  (bind _cube (`/Game/Blueprints/BP_DoorOudated.Cube` Door))
  (`SceneComponent.SetVisibility` _cube false false)
  (`PrimitiveComponent.SetCollisionEnabled` _cube "NoCollision")
  (return))

(fn `UserConstructionScript`)