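; BP_Lever is an interactable lever that toggles low gravity for the player within a separate GetCollider zone.
; Overlapping Coll shows the character's interact widget and lets its Interact flag flip the Gravity toggle.
; Tick polls both overlap states and sets the character's GravityScale, reduced only inside the zone with Gravity on.
; The Interact and Grav functions are empty, and AirControl changes are disconnected.
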(event `self.Coll.OnComponentEndOverlap`
  (params (OverlappedComponent :type "PrimitiveComponent Object Reference") (OtherActor :type "Actor Object Reference") (OtherComp :type "PrimitiveComponent Object Reference") (OtherBodyIndex :type Integer))
  (set `self.InCollider` false)
  (`/Game/ThirdPerson/Blueprints/BP_ThirdPersonCharacter.Widget_Interact_Disappear` (cast `/Game/ThirdPerson/Blueprints/BP_ThirdPersonCharacter` (`GameplayStatics.GetPlayerCharacter` 0) :!pure true) null))

(event `self.Coll.OnComponentBeginOverlap`
  (params (OverlappedComponent :type "PrimitiveComponent Object Reference") (OtherActor :type "Actor Object Reference") (OtherComp :type "PrimitiveComponent Object Reference") (OtherBodyIndex :type Integer) (bFromSweep :type Boolean) (SweepResult :type "HitResult Structure (by ref)"))
  (`|ExecutionSequence`
    (:`then_0`
      (`/Game/ThirdPerson/Blueprints/BP_ThirdPersonCharacter.Widget_Interact_Appear` (cast `/Game/ThirdPerson/Blueprints/BP_ThirdPersonCharacter` (`GameplayStatics.GetPlayerCharacter` 0) :!pure true) "/Game/Widget/WBP_InteractButton.WBP_InteractButton_C"))
    (:`then_1`
      (set `self.InCollider` (== OtherActor (`GameplayStatics.GetPlayerCharacter` 0))))))

(event `self.ReceiveTick`
  (params (DeltaSeconds :type "Float (single-precision)"))
  (`|ExecutionSequence`
    (:`then_0`
      (bind _returnvalue (`GameplayStatics.GetActorOfClass` "/Game/ThirdPerson/Blueprints/BP_ThirdPersonCharacter.BP_ThirdPersonCharacter_C")))
    (:`then_1`
      (if (`self.InCollider`)
        (if (`/Game/ThirdPerson/Blueprints/BP_ThirdPersonCharacter.Interact` _returnvalue)
          (if (`self.Gravity`)
            (set `self.Gravity` false)
            (set `/Game/ThirdPerson/Blueprints/BP_ThirdPersonCharacter.Interact` false _returnvalue)
            (else
              (set `self.Gravity` true)
              (set `/Game/ThirdPerson/Blueprints/BP_ThirdPersonCharacter.Interact` false _returnvalue))))))
    (:`then_2`
      (`|ExecutionSequence`
        (:`then_0`
          (bind _returnvalue_2 (`GameplayStatics.GetActorOfClass` "/Game/ThirdPerson/Blueprints/BP_ThirdPersonCharacter.BP_ThirdPersonCharacter_C")))
        (:`then_1`
          (if (`self.InGetCollider`)
            (if (`self.Gravity`)
              (bind _charactermovement (`Character.CharacterMovement` _returnvalue_2))
              (set `CharacterMovementComponent.GravityScale` 0.5 _charactermovement)
              (else
                (set `CharacterMovementComponent.GravityScale` 1.75 _charactermovement)))
            (else
              (set `CharacterMovementComponent.GravityScale` 1.75 _charactermovement))))))))

(event `self.GetCollider.OnActorBeginOverlap`
  (params (OverlappedActor :type "Actor Object Reference") (OtherActor :type "Actor Object Reference"))
  (set `self.InGetCollider` (== OtherActor (`GameplayStatics.GetPlayerCharacter` 0))))

(event `self.GetCollider.OnActorEndOverlap`
  (params (OverlappedActor :type "Actor Object Reference") (OtherActor :type "Actor Object Reference"))
  (set `self.InGetCollider` false))

(fn `Grav`)

(fn `Interact`)

(fn `UserConstructionScript`)