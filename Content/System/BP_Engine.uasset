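; BP_Engine is an actor whose Activate function switches the level's lights on and its red alarms off.
; Activate runs a sequence that gathers every BP_Lights actor and calls LightsOn, then gathers every BP_RedAlarm actor and calls OffAlarm.
; Targets are found by class search with no stored references, and the event graph and construction script add no logic of their own.
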(fn `Activate`
  (`|ExecutionSequence`
    (:`then_0`
      (bind _outactors (`GameplayStatics.GetAllActorsOfClass` "/Game/Blueprints/BP_Lights.BP_Lights_C"))
      (`/Game/Blueprints/BP_Lights.Lights_On` _outactors))
    (:`then_1`
      (bind _outactors_2 (`GameplayStatics.GetAllActorsOfClass` "/Game/Blueprints/BP_RedAlarm.BP_RedAlarm_C"))
      (`/Game/Blueprints/BP_RedAlarm.Off Alarm` _outactors_2))))

(fn `UserConstructionScript`
  (`parent.UserConstructionScript`))