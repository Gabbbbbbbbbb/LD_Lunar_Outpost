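; BP_InteractableSystem is an interactable with a trigger box that switches a list of linked systems on and off.
; Box overlap by the player character sets or clears that character's ObjectInArea reference and InArea flag.
; Activate and Deactivation forward the call to every SystemToActivate entry and update IsActivated inside the loop.
; Nothing in this graph calls those two functions.
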(event `self.Box.OnComponentBeginOverlap`
  (params (OverlappedComponent :type "PrimitiveComponent Object Reference") (OtherActor :type "Actor Object Reference") (OtherComp :type "PrimitiveComponent Object Reference") (OtherBodyIndex :type Integer) (bFromSweep :type Boolean) (SweepResult :type "HitResult Structure (by ref)"))
  (if (== OtherActor (`GameplayStatics.GetPlayerCharacter` 0))
    (bind _asbp_third_person_character (cast `/Game/ThirdPerson/Blueprints/BP_ThirdPersonCharacter` (`GameplayStatics.GetPlayerCharacter` 0)))
    (set `/Game/ThirdPerson/Blueprints/BP_ThirdPersonCharacter.ObjectInArea` self _asbp_third_person_character)
    (set `/Game/ThirdPerson/Blueprints/BP_ThirdPersonCharacter.InArea` true _asbp_third_person_character)))

(event `self.Box.OnComponentEndOverlap`
  (params (OverlappedComponent :type "PrimitiveComponent Object Reference") (OtherActor :type "Actor Object Reference") (OtherComp :type "PrimitiveComponent Object Reference") (OtherBodyIndex :type Integer))
  (if (== OtherActor (`GameplayStatics.GetPlayerCharacter` 0))
    (bind _asbp_third_person_character (cast `/Game/ThirdPerson/Blueprints/BP_ThirdPersonCharacter` (`GameplayStatics.GetPlayerCharacter` 0)))
    (set `/Game/ThirdPerson/Blueprints/BP_ThirdPersonCharacter.ObjectInArea` null _asbp_third_person_character)
    (set `/Game/ThirdPerson/Blueprints/BP_ThirdPersonCharacter.InArea` false _asbp_third_person_character)))

(fn `Activate`
  (for _array_element (`self.SystemToActivate`)
    (`/Game/System/BP_System.Activate` _array_element)
    (set `self.IsActivated` true)))

(fn `Deactivation`
  (for _array_element (`self.SystemToActivate`)
    (`/Game/System/BP_System.Deactivate` _array_element)
    (set `self.IsActivated` false)))

(fn `UserConstructionScript`)