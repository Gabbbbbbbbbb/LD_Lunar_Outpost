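; BP_Door is a sliding door that opens and closes by moving its Cube component.
; Activate and Deactivate print a debug string, then call the Open and Close events respectively.
; Open uses MoveComponentTo to slide the Cube along relative Y over a short time, and Close moves it back to the default zero location.
; BeginPlay, overlap and Tick are disabled, so movement runs only when those events are called.
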(event `Open`
  (`KismetSystemLibrary.MoveComponentTo` (`self.Cube`) (0.0 -550.0 0.0) (struct) false false 0.4))

(event `Close`
  (`KismetSystemLibrary.MoveComponentTo` (`self.Cube`) (0.0 0.0 0.0) (struct) false false 0.4))

(fn `Activate`
  (`KismetSystemLibrary.PrintString` "tg")
  (`self.Open`))

(fn `Deactivate`
  (`KismetSystemLibrary.PrintString` "Hello")
  (`self.Close`))

(fn `UserConstructionScript`
  (`parent.UserConstructionScript`))