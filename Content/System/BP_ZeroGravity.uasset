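; BP_ZeroGravity is an actor that switches the third-person player character between reduced gravity and a heavier gravity setting.
; Activate and Deactivate set a boolean and fire the matching event, which writes the character movement's GravityScale.
; Tick re-applies the state every frame based on that boolean, finding the character by player cast when active and by class lookup when inactive.
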(event `Activated`
  (bind _asbp_third_person_character (cast `/Game/ThirdPerson/Blueprints/BP_ThirdPersonCharacter` (`GameplayStatics.GetPlayerCharacter` 0)))
  (bind _output_get (set `CharacterMovementComponent.GravityScale` 0.5 (`Character.CharacterMovement` _asbp_third_person_character))))

(event `Deactivated`
  (bind _returnvalue (`GameplayStatics.GetActorOfClass` "/Game/ThirdPerson/Blueprints/BP_ThirdPersonCharacter.BP_ThirdPersonCharacter_C"))
  (bind _output_get (set `CharacterMovementComponent.GravityScale` 1.75 (`Character.CharacterMovement` _returnvalue))))

(event `self.ReceiveTick`
  (params (DeltaSeconds :type "Float (single-precision)"))
  (`parent.ReceiveTick` DeltaSeconds)
  (if (`self.NewVar`)
    (`self.Activated`)
    (else
      (`self.Deactivated`))))

(fn `Activate`
  (`self.Activated`)
  (set `self.NewVar` true))

(fn `Deactivate`
  (`self.Deactivated`)
  (set `self.NewVar` false))

(fn `UserConstructionScript`
  (`parent.UserConstructionScript`))