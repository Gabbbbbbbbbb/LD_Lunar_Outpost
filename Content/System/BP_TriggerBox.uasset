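; BP_TriggerBox is a trigger volume that toggles every system in SystemsToActivate on or off.
; Any actor entering the Box flips the state, while exit flips it only for the player character when WillReactOnExit is set.
; InteractableOnce blocks further toggles once activated.
; Activate and Deactivate forward the call to each system and update IsActivated inside the loop, so an empty list never changes state.
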(event `self.Box.OnComponentBeginOverlap`
  (params (OverlappedComponent :type "PrimitiveComponent Object Reference") (OtherActor :type "Actor Object Reference") (OtherComp :type "PrimitiveComponent Object Reference") (OtherBodyIndex :type Integer) (bFromSweep :type Boolean) (SweepResult :type "HitResult Structure (by ref)"))
  (bind _isactivated (`self.isActivated`))
  (if true
    (if (and (`self.InteractableOnce`) _isactivated)
      _
      (elif _isactivated
        (`self.Deactivate`)
        (else
          (`self.Activate`))))))

(event `self.Box.OnComponentEndOverlap`
  (params (OverlappedComponent :type "PrimitiveComponent Object Reference") (OtherActor :type "Actor Object Reference") (OtherComp :type "PrimitiveComponent Object Reference") (OtherBodyIndex :type Integer))
  (bind _isactivated (`self.isActivated`))
  (if (== OtherActor (`GameplayStatics.GetPlayerCharacter` 0))
    (if (`self.WillReactOnExit`)
      (if (and (`self.InteractableOnce`) _isactivated)
        _
        (elif _isactivated
          (`self.Deactivate`)
          (else
            (`self.Activate`)))))))

(fn `Activate`
  (for _array_element (`self.SystemsToActivate`)
    (`/Game/System/BP_System.Activate` _array_element)
    (set `self.IsActivated` true)))

(fn `Deactivate`
  (for _array_element (`self.SystemsToActivate`)
    (`/Game/System/BP_System.Deactivate` _array_element)
    (set `self.IsActivated` false)))

(fn `UserConstructionScript`)