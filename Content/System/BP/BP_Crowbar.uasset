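; BP_Crowbar is a crowbar pickup that the player carries on their back once it is activated.
; Activate snaps it to the Back_Socket on the third-person character's mesh, then calls CrowbarPickedUp on the BP_Vent found through GetActorOfClass.
; The event graph holds only disabled default events, so all of its behavior runs through Activate.
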(fn `Activate`
  (`self.K2_AttachToComponent` (`Character.Mesh` (cast `/Game/ThirdPerson/Blueprints/BP_ThirdPersonCharacter` (`GameplayStatics.GetPlayerCharacter` 0) :!pure true)) "Back_Socket" "SnapToTarget" "SnapToTarget" "SnapToTarget")
  (bind _returnvalue (`GameplayStatics.GetActorOfClass` "/Game/System/BP/BP_Vent.BP_Vent_C"))
  (`/Game/System/BP/BP_Vent.CrowbarPickedUp` _returnvalue))

(fn `UserConstructionScript`
  (`parent.UserConstructionScript`))